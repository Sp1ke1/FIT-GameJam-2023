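; Cannonball projectile that flies at a set velocity and explodes on a blocking hit with any actor except itself or its owner.
; Explosion hides and stops the ball, waits a damage delay, applies radius damage, then destroys the actor.
; A multi-sphere trace damages each other actor's BPAC_CM_HP component once and broadcasts OnKilledTarget for kills.
; The explosion visuals function is an empty stub, and the flight-distance check is unused.
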(event `self.ReceiveBeginPlay`
  (set `self.InitialLocation` (`SceneComponent.K2_GetComponentLocation` (`self.BallMesh`)))
  (`ProjectileMovementComponent.SetVelocityInLocalSpace` (`self.ProjectileMovement`) (`self.ProjectileVelocity`)))

(event `self.ReceiveActorBeginOverlap`
  (params (OtherActor :type "Actor Object Reference")))

(event `self.ReceiveTick`
  (params (DeltaSeconds :type "Float (single-precision)"))
  (if true
    _))

(event `self.BallMesh.OnComponentHit`
  (params (HitComponent :type "PrimitiveComponent Object Reference") (OtherActor :type "Actor Object Reference") (OtherComp :type "PrimitiveComponent Object Reference") (NormalImpulse :type "Vector Structure") (Hit :type "HitResult Structure (by ref)"))
  (bind (_bblockinghit _binitialoverlap _time _distance _location _impactpoint _normal _impactnormal _physmat _hitactor) (`GameplayStatics.BreakHitResult` Hit))
  (if _bblockinghit
    (`/Engine/EditorBlueprintResources/StandardMacros.IsValid` _hitactor
      (:`Is Valid`
        (if (and (!= _hitactor self) (!= _hitactor (`self.GetOwner`)))
          (`self.Explode`))))))

(event `Explode`
  ;[1 1 1] No impl
  (`self.SpawnExplosionVisuals`)
  (`self.HideProjectile`)
  (`KismetSystemLibrary.Delay` (`self.DamageDelay`))
  (`self.ExplosionDamageImpl`)
  (`self.K2_DestroyActor`))

(event `HideProjectile`
  (`SceneComponent.SetHiddenInGame` (`self.BallMesh`) true false)
  (`PrimitiveComponent.SetCollisionEnabled` (`self.BallMesh`) "NoCollision")
  (`ProjectileMovementComponent.StopSimulating` (`self.ProjectileMovement`) (`GameplayStatics.MakeHitResult` false)))

(fn `ExplodeImpl`
  (locals (CurrentHitActor :type "Actor Object Reference") (HitActors :type "Set of Actor Object Reference")))

(fn `ExplosionDamageImpl`
  (locals (CurrentHitActor :type "Actor Object Reference") (HitActors :type "Set of Actor Object Reference"))
  (bind _currenthitactor (`local.CurrentHitActor`))
  (bind _returnvalue (`SceneComponent.K2_GetComponentLocation` (`self.BallMesh`)))
  (bind _outhits (`KismetSystemLibrary.SphereTraceMultiForObjects` :`Start` _returnvalue :`End` (+ _returnvalue (1.0 0.0 0.0)) :`Radius` (`self.DamageRadius`) :`ObjectTypes` (`self.TraceObjectTypes`) :`DrawDebugType` (select `bool` (`self.DebugTraces`) :`true` "ForDuration" :!type "EDrawDebugTrace Enum")))
  (for _array_element _outhits
    (bind (_bblockinghit _binitialoverlap _time _distance _location _impactpoint _normal _impactnormal _physmat _hitactor) (`GameplayStatics.BreakHitResult` _array_element))
    (if _bblockinghit
      (`/Engine/EditorBlueprintResources/StandardMacros.IsValid` _hitactor
        (:`Is Valid`
          (set `local.CurrentHitActor` _hitactor)
          (if (and (!= _currenthitactor self) (!= _currenthitactor (`self.GetOwner`)))
            (bind _returnvalue_2 (`self.GetComponentByClass` _hitactor "/Game/CubeMetamorphoze/Characters/Attack/Components/BPAC_CM_HP.BPAC_CM_HP_C"))
            (`/Engine/EditorBlueprintResources/StandardMacros.IsValid` _returnvalue_2
              (:`Is Valid`
                (if (not (`BlueprintSetLibrary.Set_Contains` (`local.HitActors`) (`local.CurrentHitActor`)))
                  (`BlueprintSetLibrary.Set_Add` (`local.HitActors`) (`local.CurrentHitActor`))
                  (bind _islethal (`/Game/CubeMetamorphoze/Characters/Attack/Components/BPAC_CM_HP.ReceiveDamage` _returnvalue_2 (`self.Damage`)))
                  (if _islethal
                    (`self.OnKilledTarget` (`local.CurrentHitActor`))))))))))))

(fn `SpawnExplosionVisuals`)

(fn `UserConstructionScript`)