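; BP_Arrow is an arrow projectile that damages actors carrying a BPAC_CM_HP health component.
; ProjectileMovement launches it along its local velocity, and Tick destroys it beyond FlightDistance from its start.
; A Sphere hit ignores the owner, hides the arrow and disables collision, then applies damage after a delay.
; A true ReceiveDamage result fires OnKilledTarget before destruction, while valid targets without health destroy the arrow immediately.
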(event `self.ReceiveBeginPlay`
  (set `self.InitialLocation` (`SceneComponent.K2_GetComponentLocation` (`self.Sphere`)))
  (`ProjectileMovementComponent.SetVelocityInLocalSpace` (`self.ProjectileMovement`) (`self.ProjectileVelocity`)))

(event `self.ReceiveTick`
  (params (DeltaSeconds :type "Float (single-precision)"))
  (if (> (`KismetMathLibrary.Vector_Distance` (`SceneComponent.K2_GetComponentLocation` (`self.Sphere`)) (`self.InitialLocation`)) (`self.FlightDistance`))
    (`self.DestroyImpl`)))

(event `self.Sphere.OnComponentHit`
  (params (HitComponent :type "PrimitiveComponent Object Reference") (OtherActor :type "Actor Object Reference") (OtherComp :type "PrimitiveComponent Object Reference") (NormalImpulse :type "Vector Structure") (Hit :type "HitResult Structure (by ref)"))
  (bind _returnvalue (`self.GetComponentByClass` OtherActor "/Game/CubeMetamorphoze/Characters/Attack/Components/BPAC_CM_HP.BPAC_CM_HP_C"))
  (`/Engine/EditorBlueprintResources/StandardMacros.IsValid` OtherActor
    (:`Is Valid`
      (if (and (!= (`self.GetOwner`) OtherActor) (!= OtherActor self))
        (`/Engine/EditorBlueprintResources/StandardMacros.IsValid` _returnvalue
          (:`Is Valid`
            (`self.HideProjectile`)
            (`KismetSystemLibrary.Delay` (`self.DamageDelay`))
            (bind _islethal (`/Game/CubeMetamorphoze/Characters/Attack/Components/BPAC_CM_HP.ReceiveDamage` _returnvalue (`self.Damage`) "NewEnumerator0"))
            (if _islethal
              (`self.OnKilledTarget` OtherActor))
            (`self.DestroyImpl`))
          (:`Is Not Valid`
            (`self.DestroyImpl`)))))))

(event `DestroyImpl`
  (`self.K2_DestroyActor`))

(fn `HideProjectile`
  (`SceneComponent.SetHiddenInGame` (`self.ArrowMesh`) true false)
  (`PrimitiveComponent.SetCollisionEnabled` (`self.Sphere`) "NoCollision"))

(fn `UserConstructionScript`)